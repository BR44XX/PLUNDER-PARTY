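; BP_Goalie is a skull hockey goal that scores when a skullBall overlaps its Box component.
; On overlap it casts the actor to skullBall and gets BP_ThirdPersonGameMode.
; The Goalie variable selects whether Team 1 or Team 2 gets the point through the game mode, then the ball respawns via RespawnSkull.
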(event OnComponentBeginOverlap(Box)
  (params (OverlappedComponent :type Primitive%20Component%20Object%20Reference) (OtherActor :type Actor%20Object%20Reference) (OtherComp :type Primitive%20Component%20Object%20Reference) (OtherBodyIndex :type Integer) (bFromSweep :type Boolean) (SweepResult :type Hit%20Result%20Structure%20%28by%20ref%29))
  (bind _asskull_ball (Utilities|Casting|CastToskullBall OtherActor))
  (Variables|Default|Setskullball _asskull_ball)
  (bind _asbp_third_person_game_mode (Utilities|Casting|CastToBP_ThirdPersonGameMode (Game|GetGameMode)))
  (switch int (Variables|Default|GetGoalie)
    (:0
      (Default|AddTeam1Score _asbp_third_person_game_mode)
      (Default|RespawnSkull (Variables|Default|Getskullball)))
    (:1
      (Default|AddTeam2Score _asbp_third_person_game_mode)
      (Default|RespawnSkull (Variables|Default|Getskullball)))))

(event EventBeginPlay)

(event Collision|EventActorBeginOverlap
  (params (OtherActor :type Actor%20Object%20Reference)))

(event EventTick
  (params (DeltaSeconds :type Float%20%28single-precision%29)))

(fn ConstructionScript)